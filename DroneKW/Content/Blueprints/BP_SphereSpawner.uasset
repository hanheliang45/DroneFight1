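; BP_SphereSpawner is an actor that keeps spawning BP_Sphere actors at random points around itself.
; BeginPlay starts a looping timer that fires the Spawn event every few seconds.
; CalculateSpawnPoint offsets the actor's location along a random rotator's forward vector by a random distance up to Radius.
; A debug sphere draw showing that radius is present but disconnected, so it never runs.
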(event Custom|Spawn
  (Game|SpawnActorfromClass "/Game/Blueprints/BP_Sphere.BP_Sphere_C" (CallFunction|CalculateSpawnPoint) "Undefined" "MultiplyWithRoot" 0 0))

(event EventBeginPlay
  (Utilities|Time|SetTimerbyEvent (delegate Custom|Spawn) 3.0 true))

(fn ConstructionScript)

(fn CalculateSpawnPoint
  (return (Math|Conversions|ToTransform(Vector) (+ (Transformation|GetActorLocation) (* (Math|Vector|GetForwardVector (Math|Random|RandomRotator false)) (Math|Random|RandomFloatinRange 0.0 (Variables|Default|GetRadius)))))))