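; Drone actor that continuously flies toward and turns to face a target it treats as the player.
; BeginPlay caches the first Pawn returned by GetAllActorsOfClass as that target, without checking that it is player-controlled.
; Each Tick offsets the drone along the direction to the target at Speed without sweeping, then eases its rotation toward it with RInterpTo at Rspeed.
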(event EventBeginPlay
  (bind _outactors (Actor|GetAllActorsOfClass "/Script/Engine.Pawn"))
  (Variables|Default|SetPlayer (Utilities|Array|Get(acopy) _outactors)))

(event EventTick
  (params (DeltaSeconds :type Float%20%28single-precision%29))
  (Utilities|FlowControl|Sequence
    (:then_0
      (Transformation|AddActorWorldOffset (* (Math|Vector|Normalize (- (Transformation|GetActorLocation (Variables|Default|GetPlayer)) (Transformation|GetActorLocation)) 1.0) (* (Variables|Default|GetSpeed) (Utilities|Time|GetWorldDeltaSeconds)))))
    (:then_1
      (Transformation|SetActorRotation (Math|Interpolation|RInterpTo (Transformation|GetActorRotation) (Math|Rotator|FindLookatRotation (Transformation|GetActorLocation) (Transformation|GetActorLocation (Variables|Default|GetPlayer))) (Utilities|Time|GetWorldDeltaSeconds) (Variables|Default|GetRspeed))))))

(fn ConstructionScript)