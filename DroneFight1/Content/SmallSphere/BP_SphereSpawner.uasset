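; BP_SphereSpawner periodically spawns BP_SmallSphere actors at random points within a spherical radius around itself.
; On BeginPlay it draws a long-lived debug sphere showing the radius and starts a looping timer on SpawnTime.
; Each timer tick spawns one sphere with a random rotation.
; GetRandomPointInSphere scales a random direction by a random distance within the radius, so points cluster toward the center rather than filling the volume uniformly.
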(event Custom|SpawnSmallSphere
  (Game|SpawnActorfromClass "/Game/SmallSphere/BP_SmallSphere.BP_SmallSphere_C" (Math|Transform|MakeTransform (CallFunction|GetRandomPointinSphere) (Math|Random|RandomRotator false) "1.000000,1.000000,1.000000") "Undefined" "MultiplyWithRoot" 0 0))

(event EventBeginPlay
  (Rendering|Debug|DrawDebugSphere (Transformation|GetActorLocation) (Variables|Default|GetRadius) 12 "(R=1.000000,G=1.000000,B=1.000000,A=1.000000)" 1.8e+03)
  (Utilities|Time|SetTimerbyEvent (delegate Custom|SpawnSmallSphere) (Variables|Default|GetSpawnTime) true))

(event EventTick
  (params (DeltaSeconds :type Float%20%28single-precision%29)))

(fn ConstructionScript)

(fn GetRandomPointinSphere
  (return (+ (Transformation|GetActorLocation) (* (Math|Random|RandomFloatinRange (* (Variables|Default|GetRadius) -1.0) (Variables|Default|GetRadius)) (Math|Vector|GetForwardVector (Math|Random|RandomRotator false))))))