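; BP_SmallSphere is a short-lived sphere actor that wanders through the world and vanishes on contact with a Pawn.
; Each tick it moves along its forward vector and turns by a random spin chosen at BeginPlay, so its heading keeps changing.
; Timelines drive the mesh scale for wink-in at spawn and a guarded wink-out, triggered by the lifetime timer or Pawn overlap, that destroys the actor when finished.
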(event Custom|WinkOut
  ;[0.3175 0.3175 0.3175] WinkOut
  (if (not (Variables|Default|GetIsWinkingOut))
    (Variables|Default|SetIsWinkingOut true)
    (bind _spherescale (Timeline|WinkOutTimeline Play)
      (:Update
        (Transformation|SetWorldScale3D (Variables|Default|GetSphereMesh) (Math|Conversions|ToVector(Float) _spherescale)))
      (:Finished
        (Actor|DestroyActor)))))

(event Custom|WinkIn
  (bind _spherescale (Timeline|WinkInTimeline Play)
    (:Update
      (Transformation|SetWorldScale3D (Variables|Default|GetSphereMesh) _spherescale))))

(event Custom|OnComponentBeginOverlap_Event
  (params (OverlappedComponent :type Primitive%20Component%20Object%20Reference) (OtherActor :type Actor%20Object%20Reference) (OtherComp :type Primitive%20Component%20Object%20Reference) (OtherBodyIndex :type Integer) (bFromSweep :type Boolean) (SweepResult :type Hit%20Result%20Structure%20%28by%20ref%29))
  (if (Class|GameplayStatics|ObjectIsA OtherActor "/Script/Engine.Pawn")
    (CallFunction|WinkOut)))

(event EventBeginPlay
  (CallFunction|InitializeDetalRotation)
  ;[0.3175 0.3175 0.3175] WinkOut
  (Utilities|Time|SetTimerbyEvent (delegate Custom|WinkOut) (Variables|Default|GetLifeTime))
  (CallFunction|Winkin)
  (Collision|AssignOnComponentBeginOverlap (Variables|Default|GetSphereVolume) (delegate Custom|OnComponentBeginOverlap_Event)))

(event Collision|EventActorBeginOverlap
  (params (OtherActor :type Actor%20Object%20Reference)))

(event EventTick
  (params (DeltaSeconds :type Float%20%28single-precision%29))
  ;[1 0.1056 0.7009] Move
  (CallFunction|UpdatePostion)
  (CallFunction|UpdateRotation))

(fn ConstructionScript)

(fn InitializeDetalRotation
  (Variables|Default|SetDelta%20Rotation (* (Math|Random|RandomRotator false) (Variables|Default|GetRandomRatotionScale))))

(fn UpdatePostion
  (Transformation|AddActorWorldOffset (* (Transformation|GetActorForwardVector) (Utilities|Time|GetWorldDeltaSeconds) (Variables|Default|GetMoveSpeed))))

(fn UpdateRotation
  (Class|Actor|AddActorWorldRotation (* (Variables|Default|GetDelta%20Rotation) (Utilities|Time|GetWorldDeltaSeconds))))