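; BP_BotPawn is a player-controlled bot pawn that fires energy rifles from left and right sockets on its mesh.
; BeginPlay adds the bot's Enhanced Input mapping context, and each fire press toggles a FlipFlop so shots alternate between rifles, starting with the left.
; FireRifle spawns a blast beam actor, burst effect and rifle sound at the chosen socket.
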(event Input|EnhancedActionEvents|EnhancedInputActionIA_Fire
  (params (ActionValue :type Boolean) (ElapsedSeconds :type Float%20%28double-precision%29) (TriggeredSeconds :type Float%20%28double-precision%29) (InputAction :type Input%20Action%20Object%20Reference :default "/Game/Input/IA_Fire.IA_Fire"))
  (:Started
    (Utilities|FlowControl|FlipFlop
      (:A
        (CallFunction|FireRifle true))
      (:B
        (CallFunction|FireRifle false)))))

(event EventBeginPlay
  ;[1 1 1] Add Bot IMC
  (bind _asplayer_controller (Utilities|Casting|CastToPlayerController (Pawn|GetController)))
  (Input|AddMappingContext (PlayerController|LocalPlayerSubsystems|GetEnhancedInputLocalPlayerSubsystem _asplayer_controller) "/Game/Input/IMC_Bot.IMC_Bot" 0 "(bIgnoreAllPressedKeysUntilRelease=True,bForceImmediately=False,bNotifyUserSettings=False)"))

(fn ConstructionScript)

(fn FireRifle
  (params (isLeft :type Boolean))
  (bind _botmesh (Variables|Default|GetBotMesh))
  (if isLeft
    (LocalVariables|SetSocketName "Rifle_L")
    (else
      (LocalVariables|SetSocketName "Rifle_R")))
  (Game|SpawnActorfromClass "/Game/BlastBeam/BP_BlastBeam.BP_BlastBeam_C" (Math|Transform|MakeTransform (Transformation|GetSocketLocation _botmesh (Utilities|String|StringToName (LocalVariables|GetSocketName))) (Transformation|GetSocketRotation _botmesh (Utilities|String|StringToName (LocalVariables|GetSocketName))) "1.000000,1.000000,1.000000") "Undefined" "MultiplyWithRoot" 0 0 0)
  (Niagara|SpawnSystematLocation "/Game/VFX/NS_BeamBurst.NS_BeamBurst" (Transformation|GetSocketLocation _botmesh (Utilities|String|StringToName (LocalVariables|GetSocketName))) (Transformation|GetSocketRotation _botmesh (Utilities|String|StringToName (LocalVariables|GetSocketName))))
  (Audio|PlaySoundatLocation "/Game/Sounds/Drone/SFX_EnergyRifle.SFX_EnergyRifle" (Transformation|GetSocketLocation _botmesh (Utilities|String|StringToName (LocalVariables|GetSocketName))) "0, 0, 0" 1.0 1.0 0.0 0 0 0 0))